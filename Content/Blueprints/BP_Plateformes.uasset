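; A floating platform actor that sinks while something is inside its trigger box and rises back when it leaves.
; Box overlap events play or reverse a timeline that lerps the child actor's relative Z between its initial height and a depth set by SinkDepth.
; Every tick, a sine of game time scaled by TiltIntensity rocks the child actor equally in roll and pitch, independent of overlap.
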(event `self.ReceiveBeginPlay`
  (bind (_relativelocation_x _relativelocation_y _relativelocation_z) (`KismetMathLibrary.BreakVector` (`SceneComponent.RelativeLocation` (`self.ChildActor`))))
  ; Init platform
  (set `self.InitZ` _relativelocation_z)
  ; Sinking/recovery animation
  (bind (_direction _newtrack_0) (`Timeline|Timeline` :`NewTime` (`self.SinkSpeed`) :!via `SetNewTime` :!label _label)
    (:`Update`
      (`SceneComponent.K2_SetRelativeLocation` (`self.ChildActor`) (`KismetMathLibrary.MakeVector` 0.0 0.0 (`KismetMathLibrary.Lerp` (`self.InitZ`) (`self.TargetZ`) _newtrack_0)) false false))))

(event `self.ReceiveTick`
  (params (DeltaSeconds :type "Float (single-precision)"))
  (bind _returnvalue (* (`KismetMathLibrary.DegSin` (* (`KismetSystemLibrary.GetGameTimeInSeconds`) 100.0)) (`self.TiltIntensity`)))
  ; Tilting
  (`SceneComponent.K2_SetRelativeRotation` (`self.ChildActor`) (`KismetMathLibrary.MakeRotator` _returnvalue _returnvalue) false false))

(event `self.Box.OnComponentBeginOverlap`
  (params (OverlappedComponent :type "PrimitiveComponent Object Reference") (OtherActor :type "Actor Object Reference") (OtherComp :type "PrimitiveComponent Object Reference") (OtherBodyIndex :type Integer) (bFromSweep :type Boolean) (SweepResult :type "HitResult Structure (by ref)"))
  ; Player go on platform
  (set `self.TargetZ` (- (`self.InitZ`) (`self.SinkDepth`)))
  (goto _label))

(event `self.Box.OnComponentEndOverlap`
  (params (OverlappedComponent :type "PrimitiveComponent Object Reference") (OtherActor :type "Actor Object Reference") (OtherComp :type "PrimitiveComponent Object Reference") (OtherBodyIndex :type Integer))
  ; Player jump out of platform
  (goto _label :!via `Reverse`))

(fn `UserConstructionScript`)