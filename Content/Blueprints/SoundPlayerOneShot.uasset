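; A trigger actor that plays a one-shot sound effect the first time anything overlaps its Box.
; The overlap passes a DoOnce, loads the "settings" save as SettingSave, then after a short delay plays CannonSound at the actor's location at a fixed low volume.
; It also plays the Audio component at a volume scaled from the saved SFXSound value, fading it out about two seconds later.
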(event `self.ReceiveBeginPlay`)

(event `self.Box.OnComponentBeginOverlap`
  (params (OverlappedComponent :type "PrimitiveComponent Object Reference") (OtherActor :type "Actor Object Reference") (OtherComp :type "PrimitiveComponent Object Reference") (OtherBodyIndex :type Integer) (bFromSweep :type Boolean) (SweepResult :type "HitResult Structure (by ref)"))
  (bind _audio (`self.Audio`))
  (`/Engine/EditorBlueprintResources/StandardMacros.DoOnce` false
    (:`Completed`
      (bind _returnvalue (`GameplayStatics.LoadGameFromSlot` "settings"))
      (bind _assetting_save (cast `/Game/SaveGame/SettingSave` _returnvalue))
      (bind _output_get (set `self.As Setting Save` _assetting_save))
      (`KismetSystemLibrary.Delay` 0.2)
      (`GameplayStatics.PlaySoundAtLocation` "/Game/UI/SoundsTest/Sounds/cannonSound.cannonSound" (`self.K2_GetActorLocation`) (struct) 0.2 1.0 0.0 null null null null)
      (`AudioComponent.SetVolumeMultiplier` _audio (* (`/Game/SaveGame/SettingSave.SFXSound` _output_get) 20.0))
      (`AudioComponent.Play` _audio 0.0)
      (`KismetSystemLibrary.Delay` 2.0)
      (`AudioComponent.FadeOut` _audio 1.0 0.0 "Logarithmic"))))

(fn `UserConstructionScript`)