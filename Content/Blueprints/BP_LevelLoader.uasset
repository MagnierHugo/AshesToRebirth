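; BP_LevelLoader is a trigger volume that streams a level in and out as actors enter and leave its Box component.
; Begin overlap looks up the streaming level by PackageName and, unless it is already loaded or set to load, loads the Level soft reference asynchronously and makes it visible.
; End overlap unloads that Level without blocking; neither event filters the overlapping actor.
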(event `self.Box.OnComponentBeginOverlap`
  (params (OverlappedComponent :type "PrimitiveComponent Object Reference") (OtherActor :type "Actor Object Reference") (OtherComp :type "PrimitiveComponent Object Reference") (OtherBodyIndex :type Integer) (bFromSweep :type Boolean) (SweepResult :type "HitResult Structure (by ref)"))
  (bind _returnvalue (`GameplayStatics.GetStreamingLevel` (`self.Package Name`)))
  (if (not (or (`LevelStreaming.bShouldBeLoaded` _returnvalue) (`LevelStreaming.IsLevelLoaded` _returnvalue)))
    (`GameplayStatics.LoadStreamLevelBySoftObjectPtr` (`self.Level`) true)))

(event `self.Box.OnComponentEndOverlap`
  (params (OverlappedComponent :type "PrimitiveComponent Object Reference") (OtherActor :type "Actor Object Reference") (OtherComp :type "PrimitiveComponent Object Reference") (OtherBodyIndex :type Integer))
  (`GameplayStatics.UnloadStreamLevelBySoftObjectPtr` (`self.Level`)))

(fn `UserConstructionScript`)