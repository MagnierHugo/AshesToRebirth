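; AC_Holder is an interactable holder that stores objects the player places on it and hands them back.
; On interaction with an object in hand, it appends that object to HeldObjects and places it at the HoldPositions slot of the same index, if one is free.
; With empty hands, it forwards the interaction to the last held object and removes it, giving last-in, first-out order.
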(fn `BeginInteract`
  (returns (bWaitForEnd :type Boolean))
  (bind _heldobjects (`self.HeldObjects`))
  (bind _returnvalue (`KismetArrayLibrary.Array_Length` (`self.HeldObjects`)))
  (bind _returnvalue_2 (`KismetArrayLibrary.Array_LastIndex` _heldobjects))
  (bind _pickedupobject (`/Game/__Game/Characters/Mannequins/Blueprints/BP_FirstPersonCharacter.PickedUpObject` (`self.Player`)))
  (`/Game/__Game/Characters/Mannequins/Blueprints/BP_FirstPersonCharacter.bPickedUp` (`self.Player`)
    (:`then`
      (if (> (`KismetArrayLibrary.Array_Length` (`self.HoldPositions`)) _returnvalue)
        (bind _returnvalue_3 (`KismetArrayLibrary.Array_Add` (`self.HeldObjects`) _pickedupobject))
        (`/Game/__Game/Blueprint/Interactable/Pickupable/AC_Pickupable.Place` _pickedupobject (`|GetArrayItem` (`self.HoldPositions`) _returnvalue_3))
        (return false)))
    (:`else`
      (if (> _returnvalue 0)
        (`self.BeginInteract` (`|GetArrayItem` _heldobjects _returnvalue_2))
        (`KismetArrayLibrary.Array_Remove` _heldobjects _returnvalue_2)))))