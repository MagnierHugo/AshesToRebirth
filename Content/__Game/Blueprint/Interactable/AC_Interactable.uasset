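; Base actor component for interactable objects, handling highlight, collision toggling and interaction hooks.
; On BeginPlay it caches the owner's static and skeletal mesh lists and disables its tick.
; SetHighlight toggles custom depth rendering on those meshes, and SetCollision switches the owning actor's collision.
; BeginInteract stores the player and returns false, while the end, mouse, look and move handlers are empty stubs.
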(event `self.ReceiveBeginPlay`
  (bind _returnvalue (`self.GetOwner`))
  ; Begin
  (set `self.StaticMeshList` (`Actor.K2_GetComponentsByClass` _returnvalue "/Script/Engine.StaticMeshComponent"))
  (set `self.Skeletal Mesh Components` (`Actor.K2_GetComponentsByClass` _returnvalue "/Script/Engine.SkeletalMeshComponent"))
  (`self.SetComponentTickEnabled` false))

(event `Set Highlight`
  (params (`Highlight enable` :type Boolean))
  ; SetHighlight
  (set `self.On_Highlight` `Highlight enable`)
  (`|ExecutionSequence`
    (:`then_0`
      (for _array_element (`self.StaticMeshList`)
        (`PrimitiveComponent.SetRenderCustomDepth` _array_element (`self.On_Highlight`))))
    (:`then_1`
      (for _array_element_2 (`self.Skeletal Mesh Components`)
        (`PrimitiveComponent.SetRenderCustomDepth` _array_element_2 (`self.On_Highlight`))))))

(event `Set Collision`
  (params (`New Value` :type Boolean))
  ; Set Collision
  (`Actor.SetActorEnableCollision` (`self.GetOwner`) `New Value`))

(fn `BeginInteract`
  (params (Player :type "/Game/__Game/Characters/Mannequins/Blueprints/BP_FirstPersonCharacter Object Reference"))
  (returns (bWaitForEnd :type Boolean))
  (set `self.Player` Player)
  (return false))

(fn `EndInteract`)

(fn `OnLook`
  (params (X :type "Float (double-precision)") (Y :type "Float (double-precision)")))

(fn `OnMouseInteract`)

(fn `OnMove`
  (params (X :type "Float (double-precision)") (Y :type "Float (double-precision)")))