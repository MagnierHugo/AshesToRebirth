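; Actor component that lets the player inspect an object, moving it to the player's grab point and back to where it started.
; Beginning interaction saves the start transform, derives a constant interp speed from distance over a set time, disables collision and enables tick.
; Tick interpolates toward the inspect point or back to the saved transform, switching itself off on arrival.
; Look input rotates the owner during mouse interaction.
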(event `self.ReceiveBeginPlay`
  ; Begin
  (`parent.ReceiveBeginPlay`))

(event `self.ReceiveTick`
  (params (DeltaSeconds :type "Float (single-precision)"))
  ; Update Position & Rotation
  (if (`self.bForward`)
    (`self.MoveToInspect` DeltaSeconds)
    (else
      (`self.MoveToStart` DeltaSeconds))))

(fn `BeginInteract`
  (bind _rootcomponent (`Actor.RootComponent` (`self.GetOwner`)))
  ; Variables setup
  (set `self.StartPosition` (`SceneComponent.K2_GetComponentLocation` _rootcomponent))
  (set `self.StartRotation` (`SceneComponent.K2_GetComponentRotation` _rootcomponent))
  (set `self.InterpSpeed` (/ (`KismetMathLibrary.Vector_Distance` (`SceneComponent.K2_GetComponentLocation` (`/Game/__Game/Characters/Mannequins/Blueprints/BP_FirstPersonCharacter.ObjectPosWhenGrab` (`self.Player`))) (`self.StartPosition`)) (`self.InterpTime`)))
  (set `self.bForward` true)
  (`self.Set Collision` false)
  (`self.SetComponentTickEnabled` true))

(fn `EndInteract`
  (`self.Set Collision` true)
  (`self.SetComponentTickEnabled` true)
  (set `self.bForward` false))

(fn `MoveToInspect`
  (params (DeltaTime :type "Float (double-precision)"))
  (locals (NewPosition :type "Vector Structure"))
  (bind _output_get (set `local.NewPosition` (`KismetMathLibrary.VInterpTo_Constant` (`Actor.K2_GetActorLocation` (`self.GetOwner`)) (`self.GetInspectPosition`) DeltaTime (`self.InterpSpeed`))))
  (`Actor.K2_SetActorLocation` (`self.GetOwner`) _output_get false false)
  (if (== (`self.GetInspectPosition`) (`local.NewPosition`) :`ErrorTolerance` 0.1)
    (`self.SetComponentTickEnabled` false)))

(fn `MoveToStart`
  (params (DeltaTime :type "Float (double-precision)"))
  (locals (NewPosition :type "Vector Structure" :default (0.0 0.0 0.0)) (NewRotation :type "Rotator Structure" :default (struct)))
  (`|ExecutionSequence`
    (:`then_0`
      (bind _output_get (set `local.NewRotation` (`KismetMathLibrary.RInterpTo_Constant` (`Actor.K2_GetActorRotation` (`self.GetOwner`)) (`self.StartRotation`) DeltaTime (`self.InterpSpeed`)))))
    (:`then_1`
      (bind _output_get_2 (set `local.NewPosition` (`KismetMathLibrary.VInterpTo_Constant` (`Actor.K2_GetActorLocation` (`self.GetOwner`)) (`self.StartPosition`) DeltaTime (`self.InterpSpeed`))))
      (`Actor.K2_SetActorLocationAndRotation` (`self.GetOwner`) _output_get_2 _output_get false false)
      (if (and (== (`local.NewPosition`) (`self.StartPosition`) :`ErrorTolerance` 0.1) (== (`local.NewRotation`) (`self.StartRotation`) :`ErrorTolerance` 0.1))
        (`self.SetComponentTickEnabled` false)))))

(fn `OnLook`
  (params (X :type "Float (double-precision)") (Y :type "Float (double-precision)"))
  (set `self.Yaw` X)
  (set `self.Pitch` Y))

(fn `OnMouseInteract`
  (bind _inspectionmousespeed (`self.InspectionMouseSpeed`))
  (`Actor.K2_AddActorLocalRotation` (`self.GetOwner`) (`KismetMathLibrary.MakeRotator` 0.0 (* (`self.Pitch`) _inspectionmousespeed) (* _inspectionmousespeed (`self.Yaw`))) false false))