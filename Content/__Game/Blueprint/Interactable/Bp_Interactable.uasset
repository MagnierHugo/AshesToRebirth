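; Interactable Blueprint whose Cube can show or hide an outline highlight.
; On BeginPlay it creates a dynamic instance of the Mt_Outline material and applies it to the Cube as an overlay material.
; The ToogleHighlight event flips the OnHighlight flag and writes it to the material's ThicknessTrigger scalar parameter, switching the outline without swapping materials.
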(event `self.ReceiveBeginPlay`
  ; Begin
  (bind _returnvalue (`KismetMaterialLibrary.CreateDynamicMaterialInstance` "/Game/__Game/Mat/Mt_Outline.Mt_Outline"))
  (bind _output_get (set `self.Outliner mat ref` _returnvalue))
  (`MeshComponent.SetOverlayMaterial` (`self.Cube`) _output_get))

(event `Toogle Highlight`
  ; Toogle Highlight
  (bind _output_get (set `self.On_Highlight` (not (`self.On_Highlight`))))
  (`MaterialInstanceDynamic.SetScalarParameterValue` (`self.Outliner mat ref`) "ThicknessTrigger" (`KismetMathLibrary.Conv_BoolToDouble` _output_get)))

(fn `UserConstructionScript`)