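; Interaction component for doors, extending a parent interactable component and expecting a BP_Door owner.
; It caches the owning door on BeginPlay.
; BeginInteract calls UpdateDoor with true on both the player and the door, starts a timer and returns false.
; EndInteract only defers to the parent implementation.
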(event `self.ReceiveBeginPlay`
  (`parent.ReceiveBeginPlay`)
  (bind _asbp_door (cast `/Game/__Game/Blueprint/Interactable/Door/BP_Door` (`self.GetOwner`)))
  (set `self.As BP Door` _asbp_door))

(fn `BeginInteract`
  (returns (bWaitForEnd :type Boolean))
  (`/Game/__Game/Characters/Mannequins/Blueprints/BP_FirstPersonCharacter.UpdateDoor` (`self.Player`) true)
  (`/Game/__Game/Blueprint/Interactable/Door/BP_Door.UpdateDoor` (`self.As BP Door`) true)
  (`KismetSystemLibrary.K2_SetTimerDelegate` _)
  (return false))

(fn `EndInteract`
  (`parent.EndInteract`))