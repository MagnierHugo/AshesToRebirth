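; Actor component that lets its owning actor be picked up and placed by the player.
; BeginInteract, if the player holds nothing, registers itself on the player, attaches the owner to the player's PickupPosition with location and rotation offsets, and disables collision.
; Place moves the owner to a given transform, detaches it and clears the player's PickedUp state, without restoring collision itself.
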(fn `BeginInteract`
  (returns (bWaitForEnd :type Boolean))
  (`/Game/__Game/Characters/Mannequins/Blueprints/BP_FirstPersonCharacter.bPickedUp` (`self.Player`)
    (:`then`)
    (:`else`
      (set `/Game/__Game/Characters/Mannequins/Blueprints/BP_FirstPersonCharacter.PickedUpObject` self (`self.Player`))
      (set `/Game/__Game/Characters/Mannequins/Blueprints/BP_FirstPersonCharacter.bPickedUp` true (`self.Player`))
      (`Actor.K2_AttachToComponent` (`self.GetOwner`) (`/Game/__Game/Characters/Mannequins/Blueprints/BP_FirstPersonCharacter.PickupPosition` (`self.Player`)) "None" "KeepRelative" "KeepRelative" "KeepRelative" true)
      (`self.Set Collision` false)
      (`Actor.K2_SetActorRelativeTransform` (`self.GetOwner`) (`KismetMathLibrary.MakeTransform` (`self.PositionOffset`) (`self.RotationOffset`)) false false)
      (return false))))

(fn `Place`
  (params (NewTransform :type "Transform Structure"))
  (`Actor.K2_SetActorLocationAndRotation` (`self.GetOwner`) NewTransform_Location NewTransform_Rotation false false)
  (`Actor.K2_DetachFromActor` (`self.GetOwner`) "KeepWorld" "KeepWorld" "KeepRelative")
  (set `/Game/__Game/Characters/Mannequins/Blueprints/BP_FirstPersonCharacter.bPickedUp` false (`self.Player`)))