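; Base interactable actor that supports outline highlighting and resets to its starting transform when interaction stops.
; On BeginPlay it applies a dynamic outline material as the Cube's overlay and caches the root's world location and rotation.
; SetHighlight toggles the outline through a scalar thickness parameter.
; SetCollision switches actor collision, and StopInteraction restores the cached transform and re-enables collision.
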(event `self.ReceiveBeginPlay`
  (bind _defaultsceneroot (`self.DefaultSceneRoot`))
  ; Begin
  (bind _returnvalue (`KismetMaterialLibrary.CreateDynamicMaterialInstance` "/Game/__Game/Mat/Mt_Outline.Mt_Outline"))
  (bind _output_get (set `self.Outliner mat ref` _returnvalue))
  (`MeshComponent.SetOverlayMaterial` (`self.Cube`) _output_get)
  (set `self.StartPosition` (`SceneComponent.K2_GetComponentLocation` _defaultsceneroot))
  (set `self.StartRotation` (`SceneComponent.K2_GetComponentRotation` _defaultsceneroot)))

(event `Set Highlight`
  (params (`Highlight enable` :type Boolean))
  ; SetHighlight
  (bind _output_get (set `self.On_Highlight` `Highlight enable`))
  (`MaterialInstanceDynamic.SetScalarParameterValue` (`self.Outliner mat ref`) "ThicknessTrigger" (`KismetMathLibrary.Conv_BoolToDouble` _output_get)))

(event `SetCollision`
  (params (`New value` :type Boolean))
  ; Set Collision
  (`self.SetActorEnableCollision` `New value`))

(event `StopInteraction`
  (bind _defaultsceneroot (`self.DefaultSceneRoot`))
  ; Stop Interaction
  (`SceneComponent.K2_SetWorldLocation` _defaultsceneroot (`self.StartPosition`) false false)
  (`SceneComponent.K2_SetWorldRotation` _defaultsceneroot (`self.StartRotation`) false false)
  (`self.SetCollision` true))

(fn `UserConstructionScript`)