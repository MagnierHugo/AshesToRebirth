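; Teleport box that moves the first-person player to a preset destination when they overlap its trigger Box.
; On BeginPlay it caches the player character and the world location of the TPPosition component.
; On overlap it line traces from that location to snap the player onto the hit surface, offset by capsule half-height, or uses the raw location.
; The trace end multiplies the location by the down vector instead of adding an offset, so it is not straight down.
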(event `self.ReceiveBeginPlay`
  ; Begin
  (bind _asbp_first_person_character (cast `/Game/__Game/Characters/Mannequins/Blueprints/BP_FirstPersonCharacter` (`GameplayStatics.GetPlayerCharacter` 0)))
  (set `self.As BP First Person Character` _asbp_first_person_character)
  (set `self.NewVar_0` (`SceneComponent.K2_GetComponentLocation` (`self.TP_Position`))))

(event `self.Box.OnComponentBeginOverlap`
  (params (OverlappedComponent :type "PrimitiveComponent Object Reference") (OtherActor :type "Actor Object Reference") (OtherComp :type "PrimitiveComponent Object Reference") (OtherBodyIndex :type Integer) (bFromSweep :type Boolean) (SweepResult :type "HitResult Structure (by ref)"))
  (bind _as_bp_first_person_character (`self.As BP First Person Character`))
  (bind _newvar_0 (`self.NewVar_0`))
  ; On Box Overlap
  (if (== OtherActor (`GameplayStatics.GetPlayerCharacter` 0))
    (bind (_outhit _returnvalue) (`KismetSystemLibrary.LineTraceSingle` _newvar_0 (* (* _newvar_0 (`KismetMathLibrary.Vector_Down`)) 100.0) "TraceTypeQuery1"))
    (if _returnvalue
      (`self.K2_SetActorLocation` _as_bp_first_person_character (+ (`.ImpactPoint` (`GameplayStatics.BreakHitResult` _outhit)) (`KismetMathLibrary.MakeVector` 0.0 0.0 (`CapsuleComponent.CapsuleHalfHeight` (`Character.CapsuleComponent` (`self.As BP First Person Character`))))) false true)
      (else
        (`self.K2_SetActorLocation` _as_bp_first_person_character (`self.NewVar_0`) false false)))))

(fn `UserConstructionScript`)