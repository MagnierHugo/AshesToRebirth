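; BP_Outside_Box is a trigger volume that fades in outside atmosphere effects while something overlaps it.
; On BeginPlay it caches the level's height fog settings and the first-person character.
; Entering activates the character's soot (Suie) Niagara spawner, then after a short delay a timeline blends post process weight, fog and particle spawn rate and opacity.
; Exiting reverses the timeline, deactivating the spawner when finished.
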(event `self.ReceiveBeginPlay`
  ; Begin
  (bind _returnvalue (`GameplayStatics.GetActorOfClass` "/Script/Engine.ExponentialHeightFog"))
  (bind _output_get (set `self.ExponentialHeightFog` _returnvalue))
  (bind _component (`ExponentialHeightFog.Component` _output_get))
  (set `self.InitialFogDensity` (`ExponentialHeightFogComponent.FogDensity` _component))
  (set `self.InitialFogHeight` (`ExponentialHeightFogComponent.FogHeightFalloff` _component))
  (set `self.InitialFog Inscattering Color` (`ExponentialHeightFogComponent.FogInscatteringLuminance` _component))
  (bind _asbp_first_person_character (cast `/Game/__Game/Characters/Mannequins/Blueprints/BP_FirstPersonCharacter` (`GameplayStatics.GetPlayerCharacter` 0)))
  (set `self.As BP First Person Character` _asbp_first_person_character))

(event `self.OutSide Box.OnComponentBeginOverlap`
  (params (OverlappedComponent :type "PrimitiveComponent Object Reference") (OtherActor :type "Actor Object Reference") (OtherComp :type "PrimitiveComponent Object Reference") (OtherBodyIndex :type Integer) (bFromSweep :type Boolean) (SweepResult :type "HitResult Structure (by ref)"))
  (bind _component (`ExponentialHeightFog.Component` (`self.ExponentialHeightFog`)))
  (bind _suiespawner (`/Game/__Game/Characters/Mannequins/Blueprints/BP_FirstPersonCharacter.SuieSpawner` (`self.As BP First Person Character`)))
  ; On Overlap
  (`ActorComponent.Activate` (`/Game/__Game/Characters/Mannequins/Blueprints/BP_FirstPersonCharacter.SuieSpawner` (`self.As BP First Person Character`)) false)
  (`KismetSystemLibrary.Delay` 0.3)
  (bind (_direction _value) (`Timeline|Timeline` :`NewTime` 0.0 :!label _label)
    (:`Update`
      (set `PostProcessComponent.BlendWeight` _value (`self.PostProcess`))
      (`ExponentialHeightFogComponent.SetFogDensity` _component (`KismetMathLibrary.Lerp` (`self.InitialFogDensity`) (`self.FogDensity`) _value))
      (`ExponentialHeightFogComponent.SetFogHeightFalloff` _component (`KismetMathLibrary.Lerp` (`self.InitialFogHeight`) (`self.FogHeight`) _value))
      (`ExponentialHeightFogComponent.SetFogInscatteringColor` _component (`KismetMathLibrary.LinearColorLerp` (`self.InitialFog Inscattering Color`) (`self.FogInscateringColor`) _value))
      (`NiagaraComponent.SetVariableFloat` _suiespawner "User.SpawnRate" _value)
      (`NiagaraComponent.SetVariableFloat` _suiespawner "User.Opacity" _value))
    (:`Finished`
      (if (`|EnumEquality` _direction "Backward")
        (`ActorComponent.Deactivate` (`/Game/__Game/Characters/Mannequins/Blueprints/BP_FirstPersonCharacter.SuieSpawner` (`self.As BP First Person Character`)))))))

(event `self.OutSide Box.OnComponentEndOverlap`
  (params (OverlappedComponent :type "PrimitiveComponent Object Reference") (OtherActor :type "Actor Object Reference") (OtherComp :type "PrimitiveComponent Object Reference") (OtherBodyIndex :type Integer))
  ; On Overlap
  (goto _label :!via `Reverse`))

(fn `UserConstructionScript`)