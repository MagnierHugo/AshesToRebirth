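; Editor-placed props spawner that scatters weighted random meshes inside a debug-drawn box or capsule area, built in the Construction Script.
; A seeded random stream picks points and props, with instance count derived from area size and density, capped by MaxEntity.
; Points optionally snap to ground by downward trace and get random yaw.
; Each mesh gets one cached HISM component with configurable Pawn collision, keeping instances batched.
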(event `self.ReceiveBeginPlay`)

(fn `CheckPropInstanced`
  (params (Prop :type "StaticMesh Object Reference"))
  (returns (InstancedProp :type "HierarchicalInstancedStaticMeshComponent Object Reference"))
  (bind (_value _returnvalue) (`BlueprintMapLibrary.Map_Find` (`self.HISM_map`) Prop))
  (if _returnvalue
    (if (not (`KismetSystemLibrary.IsValid` _value))
      (bind _returnvalue_2 (`AddComponent|NODE_AddHierarchicalInstancedStaticMeshComponent-1` :!label _label))
      (`StaticMeshComponent.SetStaticMesh` _returnvalue_2 Prop)
      (if (`self.hasCollision`)
        (`PrimitiveComponent.SetCollisionResponseToChannel` _returnvalue_2 "ECC_Pawn" "ECR_Block")
        (else
          (`PrimitiveComponent.SetCollisionResponseToChannel` _returnvalue_2 "ECC_Pawn" "ECR_Ignore")))
      (`PrimitiveComponent.SetCollisionEnabled` _returnvalue_2 "QueryAndPhysics")
      (`BlueprintMapLibrary.Map_Add` (`self.HISM_map`) Prop _returnvalue_2))
    (else
      (goto _label)))
  (return _value))

(fn `Cleaning`
  (bind _hism_map (`self.HISM_map`))
  (`BlueprintMapLibrary.Map_Clear` _hism_map)
  (bind (_keypin _valuepin) (`|MapForEach` _hism_map)
    (:`then`
      (`InstancedStaticMeshComponent.ClearInstances` _valuepin))
    (:`CompletedPin`
      (return))))

(fn `GetCoeffSpawnAreaSize`
  (params (Coeff :type "Float (double-precision)" :default 2.0))
  (returns (ReturnValue :type "Vector Structure"))
  (return (`KismetMathLibrary.MakeVector` (* (.x (`self.AreaSize`)) Coeff) (* (.y (`self.AreaSize`)) Coeff) (* (.z (`self.AreaSize`)) Coeff))))

(fn `GetEntitiesQuantity`
  (returns (ReturnValue :type Integer))
  (return (`KismetMathLibrary.Clamp` (`KismetMathLibrary.FTrunc` (* (* (* (* (.x (`self.AreaSize`)) (.y (`self.AreaSize`))) (.z (`self.AreaSize`))) (`self.Density`)) (`self._stabilizer`))) 0 (`self.MaxEntity`))))

(fn `GetRandomAngle`
  (returns (ReturnValue :type "Rotator Structure"))
  (return (`KismetMathLibrary.MakeRotator` 0.0 0.0 (`KismetMathLibrary.RandomFloatInRangeFromStream` (`self._stream`) 0.0 360.0))))

(fn `GetRandomPointInCapsule`
  (returns (ReturnValue :type "Vector Structure"))
  (bind __stream (`self._stream`))
  (bind _z (.z (`self.AreaSize`)))
  (bind _returnvalue (`KismetMathLibrary.RandomFloatInRangeFromStream` __stream 0.0 360.0))
  (bind _returnvalue_2 (`KismetMathLibrary.RandomFloatInRangeFromStream` __stream 0.0 (.x (`self.AreaSize`))))
  (return (+ (`KismetMathLibrary.MakeVector` (* (`KismetMathLibrary.DegCos` _returnvalue) _returnvalue_2) (* (`KismetMathLibrary.DegSin` _returnvalue) _returnvalue_2) (`KismetMathLibrary.RandomFloatInRangeFromStream` __stream (* _z -1.0) _z)) (`self.K2_GetActorLocation`))))

(fn `GetRandomProp`
  (returns (Prop :type "StaticMesh Object Reference"))
  (for _array_element (`self.Props`)
    (bind (_prop _weight) (break `/Game/AshesToRebirth/Blueprints/S_PropData` _array_element))
    (bind _returnvalue (- (`self.RandomRoll`) _weight))
    (set `self.RandomRoll` _returnvalue)
    (if (<= _returnvalue 0.0)
      (return _prop))))

(fn `SetTotalWeight`
  (for _array_element (`self.Props`)
    (set `self.TotalWeight` (+ (`.Weight_5_6235EA244285E14784BE3A907D367249` (break `/Game/AshesToRebirth/Blueprints/S_PropData` _array_element)) (`self.TotalWeight`))))
  (return))

(fn `SnapToGround`
  (params (RandomPoint :type "Vector Structure"))
  (returns (asHit :type Boolean) (ImpactPoint :type "Vector Structure"))
  (bind _outhit (`KismetSystemLibrary.LineTraceSingle` RandomPoint (`KismetMathLibrary.MakeVector` (.x RandomPoint) (.y RandomPoint) (- (.z RandomPoint) (`self._gravity_range`))) "TraceTypeQuery1"))
  (bind (_bblockinghit _binitialoverlap _time _distance _location _impactpoint) (`GameplayStatics.BreakHitResult` _outhit))
  (return _bblockinghit _impactpoint))

(fn `SpawnInstance`
  (params (InstanceLocation :type "Vector Structure"))
  (bind _prop (`self.GetRandomProp`))
  (bind _instancedprop (`self.CheckPropInstanced` _prop))
  (if (`self.IsRandomYaw`)
    (`InstancedStaticMeshComponent.AddInstance` _instancedprop (`KismetMathLibrary.MakeTransform` InstanceLocation (`self.GetRandomAngle`)) true)
    (else
      (`InstancedStaticMeshComponent.AddInstance` _instancedprop (`KismetMathLibrary.MakeTransform` InstanceLocation) true)))
  (return))

(fn `UserConstructionScript`
  (bind _returnvalue (`self.K2_GetActorRotation`))
  (bind _returnvalue_2 (`self.GetRandomPointInCapsule`))
  (bind _returnvalue_3 (`self.K2_GetActorLocation`))
  (bind _returnvalue_4 (`KismetMathLibrary.RandomPointInBoundingBoxFromStream` (`self._stream`) (`self.K2_GetActorLocation`) (`self.AreaSize`)))
  ; Draw spawn area
  (if (`self.IsRect`)
    (`KismetSystemLibrary.DrawDebugBox` _returnvalue_3 (`self.AreaSize`) (struct :`R` 255.0 :`G` 255.0 :`A` 1.0) _returnvalue 0.0 3.0)
    (else
      (`KismetSystemLibrary.DrawDebugCapsule` _returnvalue_3 (.z (`self.AreaSize`)) (.x (`self.AreaSize`)) _returnvalue (struct :`R` 255.0 :`G` 255.0 :`A` 1.0) 0.0 3.0)))
  ; Init + refresh attributes
  (`KismetMathLibrary.SetRandomStreamSeed` (`self._stream`) (`self.Seed`))
  (`self.Cleaning`)
  (`self.SetTotalWeight`)
  (for _ (range (+ (`self.GetEntitiesQuantity`) 1))
    (set `self.RandomRoll` (`KismetMathLibrary.RandomFloatInRangeFromStream` (`self._stream`) 0.0 (`self.TotalWeight`)))
    ; Spawn in rectangle
    (if (`self.IsRect`)
      (if (`self.IsOnGround`)
        (bind (_ashit _impactpoint) (`self.SnapToGround` _returnvalue_4))
        (if _ashit
          (`self.SpawnInstance` _impactpoint))
        (else
          (`self.SpawnInstance` _returnvalue_4)))
      (else
        ; Spawn in capsule
        (if (`self.IsOnGround`)
          (bind (_ashit_2 _impactpoint_2) (`self.SnapToGround` _returnvalue_2))
          (if _ashit_2
            (`self.SpawnInstance` _impactpoint_2))
          (else
            (`self.SpawnInstance` _returnvalue_2)))))))