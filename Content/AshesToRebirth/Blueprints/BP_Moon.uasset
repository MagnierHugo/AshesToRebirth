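; BP_Moon is a moon actor that orbits in the sky.
; On BeginPlay it offsets the Moon component by OrbitOffset, then Tick yaws the whole actor by OrbitingSpeed scaled with delta time while IsOrbiting is set, swinging the moon around the actor's origin.
; A debug function that prints the player's location is present, but its call is not connected to any event.
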(event `self.ReceiveBeginPlay`
  ; Place Moon in sky
  (`SceneComponent.K2_SetRelativeLocation` (`self.Moon`) (`self.OrbitOffset`) false false))

(event `self.ReceiveTick`
  (params (DeltaSeconds :type "Float (single-precision)"))
  ; Rotate Moon
  (if (`self.bIsOrbiting`)
    (`self.K2_AddActorLocalRotation` (`KismetMathLibrary.MakeRotator` 0.0 0.0 (* DeltaSeconds (`self.OrbitingSpeed`))))))

(fn `UserConstructionScript`)