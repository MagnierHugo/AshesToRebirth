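; Trigger box actor that fades the player camera on overlap, then optionally plays a cinematic and unloads the Gameplay streaming level.
; Overlap optionally blocks first-person character input and starts a configurable camera fade, waiting out any hold before clearing it.
; The cinematic plays through a media player in a viewport widget while the level unload runs without blocking.
; Input returns when no cinematic plays, or on widget removal if gameplay stays loaded.
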(event `self.ReceiveBeginPlay`)

(event `self.Box.OnComponentBeginOverlap`
  (params (OverlappedComponent :type "PrimitiveComponent Object Reference") (OtherActor :type "Actor Object Reference") (OtherComp :type "PrimitiveComponent Object Reference") (OtherBodyIndex :type Integer) (bFromSweep :type Boolean) (SweepResult :type "HitResult Structure (by ref)"))
  (bind _returnvalue (`GameplayStatics.GetPlayerCameraManager` 0))
  (bind _asbp_first_person_character (cast `/Game/__Game/Characters/Mannequins/Blueprints/BP_FirstPersonCharacter` (`GameplayStatics.GetPlayerPawn` 0)))
  (set `self.As BP First Person Character` _asbp_first_person_character)
  (`self.Block Player Inputs`
    (:`then`
      (`self.DisableInput` (`self.As BP First Person Character`) (`GameplayStatics.GetPlayerController` 0)))
    (:`else`
      _))
  (`PlayerCameraManager.StartCameraFade` _returnvalue (`self.From Alpha`) (`self.To Alpha`) (`self.Duration`) (`self.Color`) (`self.Should Fade Audio`) (`self.Hold when Finished`))
  (`self.Hold when Finished`
    (:`then`
      (`KismetSystemLibrary.Delay` (+ (`self.HoldDuration`) (`self.Duration`)))
      (`PlayerCameraManager.StopCameraFade` _returnvalue)
      (`|ExecutionSequence`
        (:`then_0`
          (`self.bPlayCinematic`
            (:`then`
              (`self.PlayCinematic`))
            (:`else`
              (`self.EnableInputs`))))
        (:`then_1`
          (`self.UnloadGameplay`))))
    (:`else`
      (`KismetSystemLibrary.Delay` (`self.Duration`))
      (`|ExecutionSequence`
        (:`then_0`
          (`self.bPlayCinematic`
            (:`then`
              (`self.PlayCinematic`))
            (:`else`
              (`self.EnableInputs`))))
        (:`then_1`
          (`self.UnloadGameplay`))))))

(event `UnloadGameplay`
  (`self.bUnloadGameplay`
    (:`then`
      (`GameplayStatics.UnloadStreamLevelBySoftObjectPtr` "/Game/Levels/LVL_Enviro/Gameplay.Gameplay"))
    (:`else`)))

(fn `EnableInputs`
  (`self.Block Player Inputs`
    (:`then`
      (`self.EnableInput` (`self.As BP First Person Character`) (`GameplayStatics.GetPlayerController` 0)))
    (:`else`)))

(fn `PlayCinematic`
  (bind _cinematicmediaplayer (`self.CinematicMediaPlayer`))
  (bind _returnvalue (`|CreateWidget` (`self.WidgetCinematic`)))
  (`UserWidget.AddToViewport` _returnvalue 0)
  (`MediaPlayer.OpenSource` _cinematicmediaplayer (`self.CinematicMediaSource`))
  (`MediaPlayer.Play` _cinematicmediaplayer)
  (add `MediaPlayer.OnEndReached` (`self.CinematicMediaPlayer`) (`|CreateDelegate` :!event `RemoveWidgets`)))

(fn `RemoveWidgets`
  (`WidgetLayoutLibrary.RemoveAllWidgets`)
  (`self.bUnloadGameplay`
    (:`then`)
    (:`else`
      (`self.EnableInputs`))))

(fn `UserConstructionScript`)