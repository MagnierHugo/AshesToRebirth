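; Procedural column actor that assembles a randomized column from bottom, middle and top static mesh pieces.
; Randomize picks a random mesh for each slot from its list, positions the pieces around the actor origin using the height variables, then spawns the shaft.
; SpawnTroncs, also run on BeginPlay, adds copies of the middle mesh stacked at MiddleHeight intervals to reach TroncNumber segments.
; The construction script is empty.
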(event `self.ReceiveBeginPlay`
  (`self.SpawnTroncs`))

(fn `AddTronc`
  (params (Index :type Integer))
  (locals (CurrentTronc :type "StaticMeshComponent Object Reference"))
  (bind _staticmesh_middle (`self.StaticMesh_Middle`))
  (bind _returnvalue (`AddComponent|NODE_AddStaticMeshComponent-2` :`RelativeTransform` (`KismetMathLibrary.MakeTransform` (+ (`KismetMathLibrary.MakeVector` 0.0 0.0 (* Index (`self.MiddleHeight`))) (`SceneComponent.RelativeLocation` _staticmesh_middle)))))
  (`StaticMeshComponent.SetStaticMesh` _returnvalue (`StaticMeshComponent.StaticMesh` _staticmesh_middle)))

(fn `GetMeshes`
  (returns (TopMesh :type "StaticMesh Object Reference") (MiddleMesh :type "StaticMesh Object Reference") (BottomMesh :type "StaticMesh Object Reference"))
  (return (`KismetArrayLibrary.Array_Random` (`self.Top`)) (`KismetArrayLibrary.Array_Random` (`self.Middle`)) (`KismetArrayLibrary.Array_Random` (`self.Bottom`))))

(fn `Randomize`
  (bind (_topmesh _middlemesh _bottommesh) (`self.GetMeshes`))
  (`|ExecutionSequence`
    (:`then_0`
      (`StaticMeshComponent.SetStaticMesh` (`self.StaticMesh_Top`) _topmesh))
    (:`then_1`
      (`StaticMeshComponent.SetStaticMesh` (`self.StaticMesh_Middle`) _middlemesh))
    (:`then_2`
      (`StaticMeshComponent.SetStaticMesh` (`self.StaticMesh_Bottom`) _bottommesh)
      (`self.SetMeshesPosition`)
      (`self.SpawnTroncs`))))

(fn `SetMeshesPosition`
  (locals (LastColumnPosition :type "Float (double-precision)"))
  (set `local.LastColumnPosition` (* (`self.MiddleHeight`) (- (`self.TroncNumber`) 1)))
  (`SceneComponent.K2_SetRelativeLocation` (`self.StaticMesh_Bottom`) (`KismetMathLibrary.MakeVector` 0.0 0.0 (* (+ (`self.BottomHeight`) (`local.LastColumnPosition`) (`self.MiddleHeight`)) -0.5)) false false)
  (`SceneComponent.K2_SetRelativeLocation` (`self.StaticMesh_Middle`) (`KismetMathLibrary.MakeVector` 0.0 0.0 (* (`local.LastColumnPosition`) -0.5)) false false)
  (`SceneComponent.K2_SetRelativeLocation` (`self.StaticMesh_Top`) (`KismetMathLibrary.MakeVector` 0.0 0.0 (* 0.5 (+ (`self.BottomHeight`) (`local.LastColumnPosition`) (`self.MiddleHeight`)))) false false))

(fn `SpawnTroncs`
  (if (> (`self.TroncNumber`) 1)
    (for _index (range 1 (`self.TroncNumber`))
      (`self.AddTronc` _index))))

(fn `UserConstructionScript`)