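; Art tool actor that generates and manages a grid of BP_ProceduralColumn actors, centered on its own location.
; A shared Foreach Column Position macro supplies grid indices and world-axis positions from rows, columns and spacing.
; Construction prunes invalid or excess columns and repositions existing ones, while SpawnColumns separately fills missing slots with attached, randomized columns.
; Batch functions clear all columns, re-randomize them or trigger their SpawnTroncs.
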(fn `CalculateFirstPosition`
  (returns (Position :type "Vector Structure"))
  (bind (_returnvalue_x _returnvalue_y _returnvalue_z) (`KismetMathLibrary.BreakVector` (`self.K2_GetActorLocation`)))
  (return (`KismetMathLibrary.MakeVector` (+ (* (- (`self.Rows`) 1) (`self.DistanceY`) 0.5) _returnvalue_x) (- _returnvalue_y (* (- (`self.Columns`) 1) (`self.DistanceX`) 0.5)) _returnvalue_z)))

(fn `ClearColumns`
  (bind (_arrayindex _arrayelement) (`/Engine/EditorBlueprintResources/StandardMacros.ReverseForEachLoop` (`self.SpawnedColumns`))
    (:`LoopBody`
      (`self.K2_DestroyActor` _arrayelement)
      (`KismetArrayLibrary.Array_Remove` (`self.SpawnedColumns`) _arrayindex))))

(fn `RandomizeAll`
  (for _array_element (`self.SpawnedColumns`)
    (`/Game/ArtTools/ColumnGeneration/BP_ProceduralColumn.Randomize` _array_element)))

(fn `SpawnColumnAtLocation`
  (params (SpawnTransform_Location :type "Vector Structure"))
  (locals (NewColumn :type "/Game/ArtTools/ColumnGeneration/BP_ProceduralColumn Object Reference"))
  (bind _newcolumn (`local.NewColumn`))
  (bind _returnvalue (`|SpawnActorFromClass` "/Game/ArtTools/ColumnGeneration/BP_ProceduralColumn.BP_ProceduralColumn_C" (`KismetMathLibrary.MakeTransform` SpawnTransform_Location) "Undefined" "MultiplyWithRoot" null (`self.Tronc Number`) null))
  (bind _output_get (set `local.NewColumn` _returnvalue))
  (`/Engine/EditorBlueprintResources/StandardMacros.IsValid` _output_get
    (:`Is Valid`
      (`self.K2_AttachToActor` (`local.NewColumn`) self "None" "KeepWorld" "KeepRelative" "KeepRelative" true)
      (`KismetArrayLibrary.Array_Add` (`self.SpawnedColumns`) _newcolumn)
      (`/Game/ArtTools/ColumnGeneration/BP_ProceduralColumn.Randomize` _newcolumn))))

(fn `SpawnColumns`
  (bind (_index _position) (`self.Foreach Column Position`)
    (:`LoopBody`
      (if (<= (`KismetArrayLibrary.Array_Length` (`self.SpawnedColumns`)) _index)
        (`self.SpawnColumnAtLocation` _position)))))

(fn `SpawnTroncsAll`
  (for _array_element (`self.SpawnedColumns`)
    (`/Game/ArtTools/ColumnGeneration/BP_ProceduralColumn.SpawnTroncs` _array_element)))

(fn `UserConstructionScript`
  (bind _spawnedcolumns (`self.SpawnedColumns`))
  (bind _spawnedcolumns_2 (`self.SpawnedColumns`))
  (bind _returnvalue (`KismetArrayLibrary.Array_Length` _spawnedcolumns_2))
  (`|ExecutionSequence`
    (:`then_0`
      (bind (_arrayindex _arrayelement) (`/Engine/EditorBlueprintResources/StandardMacros.ReverseForEachLoop` (`self.SpawnedColumns`))
        (:`LoopBody`
          (`/Engine/EditorBlueprintResources/StandardMacros.IsValid` _arrayelement
            (:`Is Not Valid`
              (`KismetArrayLibrary.Array_Remove` (`self.SpawnedColumns`) _arrayindex))))))
    (:`then_1`
      (if (<= _returnvalue (* (`self.Rows`) (`self.Columns`)))
        (bind (_index _position) (`self.Foreach Column Position` :!label _label)
          (:`LoopBody`
            (if (> _returnvalue _index)
              (`self.K2_SetActorLocation` (`|GetArrayItem` _spawnedcolumns_2 _index) _position false false))))
        (else
          (`|ExecutionSequence`
            (:`then_0`
              (set `self.bRemoveColumns` true)
              (bind (_arrayindex_2 _arrayelement_2) (`/Engine/EditorBlueprintResources/StandardMacros.ReverseForEachLoop` _spawnedcolumns)
                (:`LoopBody`
                  (if (`self.bRemoveColumns`)
                    (`|ExecutionSequence`
                      (:`then_0`
                        (`self.K2_DestroyActor` _arrayelement_2)
                        (`KismetArrayLibrary.Array_Remove` (`self.SpawnedColumns`) _arrayindex_2))
                      (:`then_1`
                        (set `self.bRemoveColumns` (> (`KismetArrayLibrary.Array_Length` _spawnedcolumns) (* (`self.Rows`) (`self.Columns`))))))))))
            (:`then_1`
              (goto _label))))))))