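; Modular sewer corridor segment built from three BP_Corridor_256 child actors, configured by flags at construction and again on BeginPlay.
; Flags set floor and water-evacuation variants, swap or remove pieces, or add a portal mesh or door.
; RoomType replaces the pieces during construction, while Block collapses them into BP_Corridor_Destroy at BeginPlay.
; Random line traces within a box place hanging chain links and a Niagara droplet effect, with debug prints left in.
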(event `self.ReceiveBeginPlay`
  (`self.Floor`)
  (`self.Type`)
  (if (`self.Droplet`)
    (`self.Drople`))
  (if (`self.Chains`)
    (`self.Chain`))
  (if (`self.Block`)
    (`|ExecutionSequence`
      (:`then_0`
        (bind _bp_corridor_256_02 (`self.BP_Corridor_256_02`)
          (:`then`
            (`ActorComponent.K2_DestroyComponent` _bp_corridor_256_02))
          (:`else`)))
      (:`then_1`
        (bind _bp_corridor_256_03 (`self.BP_Corridor_256_03`)
          (:`then`
            (`ActorComponent.K2_DestroyComponent` _bp_corridor_256_03))
          (:`else`)))
      (:`then_2`
        (`ChildActorComponent.SetChildActorClass` (`self.BP_Corridor_256_01`) "/Game/Art/Blueprint/Sewer/BP_Corridor_Destroy.BP_Corridor_Destroy_C")))
    (elif (`self.Portal`)
      (`AddComponent|NODE_AddStaticMeshComponent-7`)
      (elif (`self.Door`)
        (`AddComponent|NODE_AddChildActorComponent-6`)))))

(fn `Chain`
  (bind _box (`self.Box`))
  (bind _returnvalue (`KismetMathLibrary.RandomPointInBoundingBox` (`SceneComponent.RelativeLocation` _box) (* (.scale (`SceneComponent.GetRelativeTransform` _box)) 25.0)))
  (bind _returnvalue_2 (+ _returnvalue (`SceneComponent.K2_GetComponentLocation` (`self.Box`))))
  (for _ (range (`self.NumberChains`))
    (bind (_outhit _returnvalue_3) (`KismetSystemLibrary.LineTraceSingle` :`Start` (- _returnvalue_2 (0.0 0.0 200.0)) :`End` (* _returnvalue_2 (1.0 1.0 10.0)) :`TraceChannel` "TraceTypeQuery1" :`DrawDebugType` "ForDuration" :`bIgnoreSelf` false))
    (for _index (range (+ (`KismetMathLibrary.FTrunc` (`KismetMathLibrary.RandomFloatInRange` 1.0 (`KismetMathLibrary.Conv_IntToDouble` (- (`self.Longueur_Max`) 1)))) 1))
      (`KismetSystemLibrary.PrintString` (`KismetStringLibrary.Conv_VectorToString` _returnvalue))
      (`KismetSystemLibrary.PrintString` (`KismetStringLibrary.Conv_BoolToString` _returnvalue_3))
      (bind (_bblockinghit _binitialoverlap _time _distance _location _impactpoint _normal _impactnormal _physmat _hitactor _hitcomponent) (`GameplayStatics.BreakHitResult` _outhit))
      (`KismetSystemLibrary.PrintString` (`KismetSystemLibrary.GetDisplayName` _hitcomponent))
      (`KismetSystemLibrary.PrintString` (`KismetStringLibrary.Conv_VectorToString` _impactpoint))
      (bind _returnvalue_4 (`KismetMathLibrary.MakeTransform` (- (+ (`KismetMathLibrary.MakeVector` 0.0 0.0 (`KismetMathLibrary.Conv_IntToDouble` (* (- _index 1) -65))) _impactpoint) (`self.K2_GetActorLocation`)) (struct :`Pitch` -90.0)))
      (`KismetSystemLibrary.PrintString` (`KismetStringLibrary.Conv_TransformToString` _returnvalue_4))
      (bind _returnvalue_5 (`AddComponent|NODE_AddChildActorComponent-2` :`RelativeTransform` _returnvalue_4))
      (`KismetSystemLibrary.PrintString` (`KismetStringLibrary.Conv_VectorToString` (`SceneComponent.K2_GetComponentLocation` _returnvalue_5)))))
  (return))

(fn `Drople`
  (bind _box (`self.Box`))
  (bind _location (.location (`KismetMathLibrary.Conv_VectorToTransform` (`KismetMathLibrary.RandomPointInBoundingBox` (`SceneComponent.RelativeLocation` _box) (* (.scale (`SceneComponent.GetRelativeTransform` _box)) (10.0 10.0 0.0))))))
  (bind _outhit (`KismetSystemLibrary.LineTraceSingle` _location (+ _location (0.0 0.0 150.0)) "TraceTypeQuery1"))
  (`AddComponent|NODE_AddNiagaraComponent-0` :`RelativeTransform` (`KismetMathLibrary.MakeTransform` (+ (0.0 0.0 0.0) (`.Location` (`GameplayStatics.BreakHitResult` _outhit))) (struct :`Pitch` -90.0)))
  (`KismetSystemLibrary.PrintString` "Hello")
  (return))

(fn `Evacuation`
  (if (`self.Evacuation_water`)
    (bind _asbp_corridor_256 (cast `/Game/Art/Blueprint/Sewer/BP_Corridor_256` (`ChildActorComponent.ChildActor` (`self.BP_Corridor_256_02`))))
    (`/Game/Art/Blueprint/Sewer/BP_Corridor_256.Rotate` _asbp_corridor_256 (`self.Evacuation_water`)))
  (return))

(fn `Floor`
  (bind _flatfloor (`self.FlatFloor`))
  (if (`self.FlatFloor`)
    (bind _asbp_corridor_256 (cast `/Game/Art/Blueprint/Sewer/BP_Corridor_256` (`ChildActorComponent.ChildActor` (`self.BP_Corridor_256_01`))))
    (`/Game/Art/Blueprint/Sewer/BP_Corridor_256.Floor` _asbp_corridor_256 _flatfloor)
    (bind _asbp_corridor_256_2 (cast `/Game/Art/Blueprint/Sewer/BP_Corridor_256` (`ChildActorComponent.ChildActor` (`self.BP_Corridor_256_02`))))
    (`/Game/Art/Blueprint/Sewer/BP_Corridor_256.Floor` _asbp_corridor_256_2 _flatfloor)
    (bind _asbp_corridor_256_3 (cast `/Game/Art/Blueprint/Sewer/BP_Corridor_256` (`ChildActorComponent.ChildActor` (`self.BP_Corridor_256_03`))))
    (`/Game/Art/Blueprint/Sewer/BP_Corridor_256.Floor` _asbp_corridor_256_3 _flatfloor)
    (else
      (`self.Evacuation`)))
  (return))

(fn `Room`
  (`ActorComponent.K2_DestroyComponent` (`self.BP_Corridor_256_01`))
  (`ActorComponent.K2_DestroyComponent` (`self.BP_Corridor_256_02`))
  (`ActorComponent.K2_DestroyComponent` (`self.BP_Corridor_256_03`))
  (`AddComponent|NODE_AddChildActorComponent-8` :`RelativeTransform` (`KismetMathLibrary.MakeTransform` (0.0 0.0 0.0))))

(fn `Type`
  (if (`self.SecondType`)
    (if (`self.FlatFloor`)
      (`ActorComponent.K2_DestroyComponent` (`self.BP_Corridor_256_02`))
      (`ActorComponent.K2_DestroyComponent` (`self.BP_Corridor_256_03`))
      (`ChildActorComponent.SetChildActorClass` (`self.BP_Corridor_256_01`) null)
      (else
        (`ChildActorComponent.SetChildActorClass` (`self.BP_Corridor_256_01`) "/Game/Art/Blueprint/Sewer/BP_Corridor_02.BP_Corridor_02_C"))))
  (return))

(fn `UserConstructionScript`
  (`self.Floor`)
  (`self.Type`)
  (if (`self.Droplet`)
    (`self.Drople`))
  (if (`self.Chains`)
    (`self.Chain`))
  (if (`self.RoomType`)
    (`self.Room`)
    (elif (`self.Portal`)
      (`AddComponent|NODE_AddStaticMeshComponent-0`)
      (elif (`self.Door`)
        (`AddComponent|NODE_AddChildActorComponent-5`)))))