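; Modular sewer corridor piece that configures its floor and wall meshes in the construction script from two toggles, FlatFloor and Evacuation.
; Evacuation swaps the floor to a corner mesh, adjusts its transform, raises the wall and adds another static mesh component; otherwise the base layout is restored.
; FlatFloor lowers and turns the floor, but the following Rotate step overwrites that transform in both branches.
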(fn `Floor`
  (params (`Flat Floor` :type Boolean))
  (if `Flat Floor`
    (`SceneComponent.K2_SetRelativeTransform` (`self.SM_FloorSewer_Type1_Base`) (`KismetMathLibrary.MakeTransform` (0.0 0.0 -32.0) (struct :`Pitch` 180.0)) false false)
    (return)))

(fn `Rotate`
  (params (FinEgout :type Boolean))
  (if FinEgout
    (`StaticMeshComponent.SetStaticMesh` (`self.SM_FloorSewer_Type1_Base`) "/Game/Art/Asset/Modular/Sewer/SM_FloorSewer_Type1_Corner.SM_FloorSewer_Type1_Corner")
    (`SceneComponent.K2_SetRelativeTransform` (`self.SM_FloorSewer_Type1_Base`) (`KismetMathLibrary.MakeTransform` (0.0 -16.573267 0.0) (struct) (1.05 1.139032 1.0)) false false)
    (`SceneComponent.K2_SetRelativeLocation` (`self.SM_WallSewerType1_Base1`) (96.0 0.0 32.0) false false)
    (`AddComponent|NODE_AddStaticMeshComponent-0` :`RelativeTransform` (`KismetMathLibrary.MakeTransform` (224.0 -14.265061 0.0) (struct :`Yaw` 90.0 :`Roll` 180.0) (1.390518 1.0 1.0)))
    (else
      (`SceneComponent.K2_SetRelativeTransform` (`self.SM_FloorSewer_Type1_Base`) (`KismetMathLibrary.MakeTransform` (0.0 0.0 0.0)) false false)
      (`StaticMeshComponent.SetStaticMesh` (`self.SM_FloorSewer_Type1_Base`) "/Game/Art/Asset/Modular/Sewer/SM_FloorSewer_Type1_Base.SM_FloorSewer_Type1_Base")
      (`SceneComponent.K2_SetRelativeLocation` (`self.SM_WallSewerType1_Base1`) (96.0 0.0 0.0) false false)))
  (return))

(fn `UserConstructionScript`
  (`self.Floor` (`self.FlatFloor`))
  (`self.Rotate` (`self.Evacuation`)))