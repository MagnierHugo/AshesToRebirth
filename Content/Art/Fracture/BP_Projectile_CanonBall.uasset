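; Cannonball projectile actor for fracture scenes that spawns a physics field and pushes what it hits.
; On sphere overlap, it spawns an FS_MasterFieldArt field actor from the sphere's relative transform with enlarged scale.
; It then applies an impulse at its location to the overlapped component, scaled from its velocity by Force, and destroys itself after a long delay.
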(event `self.ReceiveTick`
  (params (DeltaSeconds :type "Float (single-precision)"))
  (`parent.ReceiveTick` DeltaSeconds))

(event `self.Sphere.OnComponentBeginOverlap`
  (params (OverlappedComponent :type "PrimitiveComponent Object Reference") (OtherActor :type "Actor Object Reference") (OtherComp :type "PrimitiveComponent Object Reference") (OtherBodyIndex :type Integer) (bFromSweep :type Boolean) (SweepResult :type "HitResult Structure (by ref)"))
  (`self.Start` (`SceneComponent.GetRelativeTransform` (`self.Sphere`)))
  (if true
    (`PrimitiveComponent.AddImpulseAtLocation` OtherComp (* (`self.GetVelocity`) (`self.Force`)) (`self.K2_GetActorLocation`) "None")
    (`KismetSystemLibrary.Delay` 145.0)
    (`self.K2_DestroyActor`)))

(event `Start`
  (params (SpawnTransform :type "Transform Structure"))
  (`|SpawnActorFromClass` "/Game/Art/Fracture/FS_MasterFieldArt.FS_MasterFieldArt_C" (`KismetMathLibrary.MakeTransform` (.location SpawnTransform) (.rotation SpawnTransform) (+ (`KismetMathLibrary.MakeVector` (.x (.scale SpawnTransform)) (.y (.scale SpawnTransform)) (.z (.scale SpawnTransform))) 20.0)) "Undefined" "MultiplyWithRoot" null null))

(fn `UserConstructionScript`
  (`parent.UserConstructionScript`))